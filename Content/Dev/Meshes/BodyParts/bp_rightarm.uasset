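; Severed right arm gore actor that ragdolls, bleeds and then removes itself.
; On BeginPlay it simulates physics with an upward impulse at the upper arm, then after a short delay spawns a blood decal and attached Niagara effect at that socket.
; A timeline spawns a fading blood decal on each update, sized by its track, and the update chain destroys the actor after a delay.
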(event `self.ReceiveBeginPlay`
  (bind _returnvalue (`SceneComponent.GetSocketLocation` (`self.SkeletalMesh`) "upperarm_r"))
  (bind (_returnvalue_x _returnvalue_y) (`KismetMathLibrary.BreakVector` (`SceneComponent.GetSocketLocation` (`self.SkeletalMesh`) "upperarm_r")))
  (`PrimitiveComponent.SetSimulatePhysics` (`self.SkeletalMesh`) true)
  (`PrimitiveComponent.AddImpulse` (`self.SkeletalMesh`) (0.0 0.0 500.0) "upperarm_r" false)
  (`KismetSystemLibrary.Delay` 1.5)
  (`GameplayStatics.SpawnDecalAtLocation` "/Game/Dev/Blood/M_Blood.M_Blood" (15.0 15.0 15.0) _returnvalue (struct :`Pitch` -90.0) 20.0)
  (`NiagaraFunctionLibrary.SpawnSystemAttached` "/Game/StarterContent/Particles/NS_BloodDeneme.NS_BloodDeneme" (`self.SkeletalMesh`) "upperarm_r" _returnvalue (* (`KismetMathLibrary.Conv_VectorToRotator` _returnvalue) -1.0) "KeepWorldPosition")
  (bind (_direction _newtrack_0) (`Timeline|decalscale` :!via `PlayFromStart`)
    (:`Update`
      (bind _returnvalue_2 (`GameplayStatics.SpawnDecalAtLocation` "/Game/Dev/Blood/M_Blood.M_Blood" _newtrack_0 (`KismetMathLibrary.MakeVector` _returnvalue_x _returnvalue_y)))
      (`DecalComponent.SetFadeOut` _returnvalue_2 0.0 7.0 true)
      (`KismetSystemLibrary.Delay` 20.0)
      (`self.K2_DestroyActor`))))

(fn `UserConstructionScript`)