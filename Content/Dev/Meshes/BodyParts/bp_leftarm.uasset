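; Severed left arm gib actor that falls under physics and bleeds before removing itself.
; On BeginPlay it simulates physics, launches upward with an impulse at the upper arm bone, then after a short delay spawns a blood decal and attached Niagara effect there.
; A timeline then spawns a timeline-sized, fading blood decal on every update at that socket's X/Y.
; A delay started from those updates later destroys the actor.
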(event `self.ReceiveBeginPlay`
  (bind (_returnvalue_x _returnvalue_y) (`KismetMathLibrary.BreakVector` (`SceneComponent.GetSocketLocation` (`self.SkeletalMesh`) "upperarm_l")))
  (bind _returnvalue (`SceneComponent.GetSocketLocation` (`self.SkeletalMesh`) "upperarm_l"))
  (bind _returnvalue_2 (`KismetMathLibrary.Conv_VectorToRotator` _returnvalue))
  (`PrimitiveComponent.SetSimulatePhysics` (`self.SkeletalMesh`) true)
  (`PrimitiveComponent.AddImpulse` (`self.SkeletalMesh`) (0.0 0.0 500.0) "upperarm_l" false)
  (`KismetSystemLibrary.Delay` 1.5)
  (`GameplayStatics.SpawnDecalAtLocation` "/Game/Dev/Blood/M_Blood.M_Blood" (15.0 15.0 15.0) _returnvalue _returnvalue_2)
  (`NiagaraFunctionLibrary.SpawnSystemAttached` "/Game/StarterContent/Particles/NS_BloodDeneme.NS_BloodDeneme" (`self.SkeletalMesh`) "upperarm_l" _returnvalue (* _returnvalue_2 -1.0) "KeepWorldPosition")
  (bind (_direction _newtrack_0) (`Timeline|Timeline` :!via `PlayFromStart`)
    (:`Update`
      (bind _returnvalue_3 (`GameplayStatics.SpawnDecalAtLocation` "/Game/Dev/Blood/M_Blood.M_Blood" _newtrack_0 (`KismetMathLibrary.MakeVector` _returnvalue_x _returnvalue_y)))
      (`DecalComponent.SetFadeOut` _returnvalue_3 0.0 7.0 true)
      (`KismetSystemLibrary.Delay` 20.0)
      (`self.K2_DestroyActor`))))

(fn `UserConstructionScript`)