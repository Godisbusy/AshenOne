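; BP_Katana is a katana weapon actor that attaches itself to the combat character that owns it.
; On BeginPlay it casts its owner to BP_CombatCharacterBase and snaps its StaticMesh component to the KatanaAttachSocket on that character's mesh.
; If the owner is not a combat character, no attachment happens; the actor has no other active logic.
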(event `self.ReceiveBeginPlay`
  (`parent.ReceiveBeginPlay`)
  (bind _asbp_combat_character_base (cast `/Game/Dev/Blueprints/BP_CombatCharacterBase` (`self.GetOwner`)))
  (`SceneComponent.K2_AttachToComponent` (`self.StaticMesh`) (`Character.Mesh` _asbp_combat_character_base) "KatanaAttachSocket" "SnapToTarget" "SnapToTarget" "SnapToTarget" true))

(fn `UserConstructionScript`
  (`parent.UserConstructionScript`))