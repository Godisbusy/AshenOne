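; BP_BaseEquipable is a base actor for equippable items that attach to a character.
; It carries static and skeletal mesh components, with GetItemMesh returning the static one when it has a mesh set, otherwise the skeletal one.
; Equipping sets the IsEquipped flag and snaps the item to AttachSocketName on the owning Character's mesh.
; Unequipping only clears the flag, without detaching, and the event graph is empty.
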(fn `AttachActor`
  (params (SocketName :type Name))
  (bind _ascharacter (cast `Character` (`self.GetOwner`)))
  (`self.K2_AttachToComponent` (`Character.Mesh` _ascharacter) SocketName "SnapToTarget" "SnapToTarget" "SnapToTarget"))

(fn `GetItemMesh`
  (returns (ItemMesh :type "PrimitiveComponent Object Reference"))
  (`/Engine/EditorBlueprintResources/StandardMacros.IsValid` (`StaticMeshComponent.StaticMesh` (`self.ItemMesh`))
    (:`Is Valid`
      (return (`self.ItemMesh`)))
    (:`Is Not Valid`
      (return (`self.ItemSkeletalMesh`)))))

(fn `IsEquipped_?`
  (returns (`isEquipped?` :type Boolean))
  (return (`self.isEquipped?`)))

(fn `OnEquipped`
  (set `self.isEquipped?` true)
  (`self.AttachActor` (`self.AttachSocketName`)))

(fn `OnUnequipped`
  (if (`self.isEquipped?`)
    (set `self.isEquipped?` false)))

(fn `SetIsEquipped`
  (params (`isEquipped?` :type Boolean))
  (set `self.isEquipped?` `isEquipped?`))

(fn `UserConstructionScript`)