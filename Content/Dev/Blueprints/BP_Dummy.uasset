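; Damageable dummy character that loses body parts when specific bones are hit.
; On damage, after the parent handling, it matches the hit bone against BoneNames, hides it and spawns the BodyPart actor of the same index at that bone's transform.
; It attaches Niagara blood: left and right bones use the preceding bone by index with oppositely signed yaw, others the hit bone itself.
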(event `self.PerformDead`
  (`parent.PerformDead`))

(event `self.ReceiveDamage`
  (params (Damage :type "Float (double-precision)") (DamageType :type "DamageType Object Reference") (`Hit Location` :type "Vector Structure") (HitNormal :type "Vector Structure") (`hit info` :type "HitResult Structure") (`Hit Component` :type "PrimitiveComponent Object Reference") (`Bone Name` :type Name) (`intigated by` :type "Controller Object Reference") (`Damage Causer` :type "Actor Object Reference"))
  (bind _mesh (`self.Mesh`))
  (bind _mesh_2 (`self.Mesh`))
  (bind _mesh_3 (`self.Mesh`))
  (bind _mesh_4 (`self.Mesh`))
  (bind _mesh_5 (`self.Mesh`))
  (bind _hitted_bone_name (`self.Hitted Bone Name`))
  (bind _mesh_6 (`self.Mesh`))
  (bind _hitted_bone_name_2 (`self.Hitted Bone Name`))
  (bind _returnvalue (`SkinnedMeshComponent.GetBoneName` _mesh_4 (- (`SkinnedMeshComponent.GetBoneIndex` _mesh_5 (`self.Hitted Bone Name`)) 1)))
  (bind _returnvalue_2 (`SkinnedMeshComponent.GetBoneName` _mesh_2 (- (`SkinnedMeshComponent.GetBoneIndex` _mesh_3 (`self.Hitted Bone Name`)) 1)))
  (bind (_returnvalue_roll _returnvalue_pitch _returnvalue_yaw) (`KismetMathLibrary.BreakRotator` (`SceneComponent.GetSocketRotation` _mesh_4 _returnvalue)))
  (bind (_returnvalue_roll_2 _returnvalue_pitch_2 _returnvalue_yaw_2) (`KismetMathLibrary.BreakRotator` (`SceneComponent.GetSocketRotation` _mesh_2 _returnvalue_2)))
  (`parent.ReceiveDamage` Damage DamageType `Hit Location` HitNormal `hit info` `Hit Component` `Bone Name` `intigated by` `Damage Causer`)
  (set `self.Hitted Bone Name` `Bone Name`)
  (for (_array_element _array_index) (`self.Bone Names`)
    (if (== _array_element (`self.Hitted Bone Name`))
      (`SkinnedMeshComponent.HideBoneByName` _mesh _hitted_bone_name "PBO_None")
      (`|SpawnActorFromClass` (`|GetArrayItem` (`self.BodyPart`) _array_index) (`SceneComponent.GetSocketTransform` _mesh _hitted_bone_name "RTS_World") "AlwaysSpawn" "MultiplyWithRoot" self self)
      (if (`KismetArrayLibrary.Array_Contains` (`self.Bone Names Right`) (`self.Hitted Bone Name`))
        (`NiagaraFunctionLibrary.SpawnSystemAttached` "/Game/StarterContent/Particles/NS_BloodDeneme.NS_BloodDeneme" _mesh_3 _returnvalue_2 (`SceneComponent.GetSocketLocation` _mesh_2 _returnvalue_2) (`KismetMathLibrary.MakeRotator` 0.0 0.0 (* _returnvalue_yaw_2 -1.0)) "KeepWorldPosition")
        (elif (`KismetArrayLibrary.Array_Contains` (`self.Bone Names Left`) (`self.Hitted Bone Name`))
          (`NiagaraFunctionLibrary.SpawnSystemAttached` "/Game/StarterContent/Particles/NS_BloodDeneme.NS_BloodDeneme" _mesh_5 _returnvalue (`SceneComponent.GetSocketLocation` _mesh_4 _returnvalue) (`KismetMathLibrary.MakeRotator` 0.0 0.0 (* _returnvalue_yaw 1.0)) "KeepWorldPosition")
          (else
            (`NiagaraFunctionLibrary.SpawnSystemAttached` "/Game/StarterContent/Particles/NS_BloodDeneme.NS_BloodDeneme" _mesh_6 _hitted_bone_name_2 (`SceneComponent.GetSocketLocation` _mesh_6 _hitted_bone_name_2) (struct) "KeepWorldPosition")))))))

(fn `UserConstructionScript`
  (`parent.UserConstructionScript`))