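; Collision component that detects hits along a mesh, such as a weapon, between start and end sockets while activated.
; Each Tick while enabled, it runs a multi-sphere object trace between the sockets and broadcasts OnHit for each valid actor.
; Activation clears the already-hit list, so each actor registers once until the list is cleared.
; Ignore lists and gameplay tags filter targets, and debug prints show hit actor and bone names.
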(event `Set Collision Mesh`
  (params (`Collision Mesh Component` :type "PrimitiveComponent Object Reference"))
  ;[1 1 1] Set Collision Mesh
  (set `self.Collision Mesh Component` `Collision Mesh Component`))

(event `ActivateCollision`
  ;[1 1 1] EnableCollision
  (`self.ClearHitActors`)
  (set `self.isCollisionEnabled?` true))

(event `DeactivateCollision`
  ;[1 1 1] DeactivateCollision
  (set `self.isCollisionEnabled?` false))

(event `ClearHitActors`
  ;[1 1 1] Clear Hit Actors
  (`KismetArrayLibrary.Array_Clear` (`self.AlreadyHitActors`)))

(event `self.ReceiveTick`
  (params (DeltaSeconds :type "Float (single-precision)"))
  (if (`self.isCollisionEnabled?`)
    (`self.CollisionTrace`)))

(event `CollisionTrace`
  (bind _collision_mesh_component (`self.Collision Mesh Component`))
  (bind _outhits (`KismetSystemLibrary.SphereTraceMultiForObjects` (`SceneComponent.GetSocketLocation` _collision_mesh_component (`self.StartSocketName`)) (`SceneComponent.GetSocketLocation` _collision_mesh_component (`self.EndSocketName`)) (`self.TraceRadius`) (`self.Object Types`) false (`self.Actors to Ignore`) (`self.Draw Debug Type`) true (struct :`R` 1.0 :`A` 1.0) (struct :`G` 1.0 :`A` 1.0) 2.0))
  (for _array_element _outhits
    (bind _output_get (set `self.LastHit` _array_element))
    (bind (_bblockinghit _binitialoverlap _time _distance _location _impactpoint _normal _impactnormal _physmat _hitactor _hitcomponent _hitbonename) (`GameplayStatics.BreakHitResult` _output_get))
    (if (`self.CanHitActor?` _hitactor)
      (`|ExecutionSequence`
        (:`then_0`
          (bind _output_get_2 (set `self.Hit Actor` _hitactor))
          (`KismetSystemLibrary.PrintString` (`KismetSystemLibrary.GetDisplayName` _output_get_2))
          (`KismetArrayLibrary.Array_Add` (`self.AlreadyHitActors`) _output_get_2)
          (`self.OnHit` (`self.LastHit`)))
        (:`then_1`
          (`KismetSystemLibrary.PrintString` (`KismetStringLibrary.Conv_NameToString` _hitbonename)))))))

(fn `AddActorToIgnore`
  (params (inActor :type "Actor Object Reference"))
  (`KismetArrayLibrary.Array_AddUnique` (`self.Actors to Ignore`) inActor))

(fn `CanHitActor?`
  (params (InActor :type "Actor Object Reference"))
  (returns (ReturnValue :type Boolean))
  (bind _returnvalue (message `/Game/Dev/Blueprints/Interfaces/BPI_GamePlayTags.GetOwnedGamePlayTags` InActor))
  (return (and (not (`KismetArrayLibrary.Array_Contains` (`self.AlreadyHitActors`) InActor)) (not (`BlueprintGameplayTagLibrary.HasAnyTags` _returnvalue (`self.GamePlayTagsToignore`) true)) (not (`KismetArrayLibrary.Array_Contains` (`self.ActorsToIgnore`) (`GameplayStatics.GetObjectClass` InActor))))))

(fn `GetActorsToIgnore`
  (returns (`Actors to Ignore` :type "Array of Actor Object Reference"))
  (return (`self.Actors to Ignore`)))

(fn `GetAlreadyHitActors`
  (returns (AlreadyHitActors :type "Array of Actor Object Reference"))
  (return (`self.AlreadyHitActors`)))

(fn `GetCollisionMeshComponent`
  (returns (`Collision Mesh Component` :type "PrimitiveComponent Object Reference"))
  (return (`self.Collision Mesh Component`)))

(fn `GetLastHit`
  (returns (LastHit :type "HitResult Structure"))
  (return (`self.LastHit`)))

(fn `isCollisionEnabled`
  (returns (`isCollisionEnabled?` :type Boolean))
  (return (`self.isCollisionEnabled?`)))

(fn `RemoveActorToIgnore`
  (params (`ınRemoveActor` :type "Actor Object Reference"))
  (`KismetArrayLibrary.Array_RemoveItem` (`self.Actors to Ignore`) `ınRemoveActor`))