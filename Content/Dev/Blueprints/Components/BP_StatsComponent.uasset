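; Character stats component that tracks base, max and current values per stat, handling damage and stamina regeneration.
; Current values are seeded from the base map, and changes broadcast an update event, with modifications clamped between zero and max.
; Stamina regeneration restarts after a retriggerable delay on a looping timer until full; other stats do not regenerate.
; Damage is scaled down by Armor, and zero Health sets the owner's state component to Dead.
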(event `StartRegen`
  (params (StatType :type "/Game/Dev/Blueprints/Enums/E_Stats Enum" :default "NewEnumerator0"))
  (switch `/Game/Dev/Blueprints/Enums/E_Stats` StatType
    (:`NewEnumerator2`
      (`KismetSystemLibrary.K2_ClearTimer` null "RegenStamina")
      (`KismetSystemLibrary.RetriggerableDelay` 1.0)
      (`KismetSystemLibrary.K2_SetTimer` null "RegenStamina" 0.1 true))))

(fn `GetBaseStatValue`
  (params (stat :type "/Game/Dev/Blueprints/Enums/E_Stats Enum" :default "NewEnumerator0"))
  (returns (`Base Value` :type "Float (double-precision)"))
  (return (break `/Game/Dev/Blueprints/Structs/F_BaseStats` (`BlueprintMapLibrary.Map_Find` (`self.BaseStats`) stat))))

(fn `GetCurrentStatValue`
  (params (stat :type "/Game/Dev/Blueprints/Enums/E_Stats Enum" :default "NewEnumerator0"))
  (returns (Value :type "Float (double-precision)"))
  (return (`BlueprintMapLibrary.Map_Find` (`self.CurrentStats`) stat)))

(fn `GetMaxStatValue`
  (params (stat :type "/Game/Dev/Blueprints/Enums/E_Stats Enum" :default "NewEnumerator0"))
  (returns (`Max Value` :type "Float (double-precision)"))
  (return (`.MaxValue_5_DF4519844F1FD56588421A849EB5E8C7` (break `/Game/Dev/Blueprints/Structs/F_BaseStats` (`BlueprintMapLibrary.Map_Find` (`self.BaseStats`) stat)))))

(fn `InitializeStats`
  (bind _keys (`BlueprintMapLibrary.Map_Keys` (`self.BaseStats`)))
  (for _array_element _keys
    (`self.SetCurrentStatValue` _array_element (break `/Game/Dev/Blueprints/Structs/F_BaseStats` (`BlueprintMapLibrary.Map_Find` (`self.BaseStats`) _array_element)))))

(fn `ModifyCurrentStatValue`
  (params (Stat :type "/Game/Dev/Blueprints/Enums/E_Stats Enum" :default "NewEnumerator0") (Value :type "Float (double-precision)") (`bShouldRegenerate?` :type Boolean))
  (locals (LValue :type "Float (double-precision)"))
  (bind _stat (`local.Stat`))
  (if (!= Value 0.0)
    (bind _output_get (set `local.LValue` (+ (`self.GetCurrentStatValue` Stat) Value)))
    (bind _output_get_2 (set `local.LValue` (`KismetMathLibrary.FClamp` _output_get 0.0 (`self.GetMaxStatValue` (`local.Stat`)))))
    (`self.SetCurrentStatValue` _stat _output_get_2)
    (if (`local.bShouldRegenerate?`)
      (`self.StartRegen` _stat))))

(fn `RegenStamina`
  (`self.SetCurrentStatValue` "NewEnumerator2" (`KismetMathLibrary.FClamp` (+ (`self.GetCurrentStatValue` "NewEnumerator2") (`self.StaminaRegenRate`)) 0.0 (`self.GetMaxStatValue` "NewEnumerator2")))
  (if (>= (`self.GetCurrentStatValue` "NewEnumerator2") (`self.GetMaxStatValue` "NewEnumerator2"))
    (`KismetSystemLibrary.K2_ClearTimer` null "RegenStamina")))

(fn `SetBaseStatValue`
  (params (stat :type "/Game/Dev/Blueprints/Enums/E_Stats Enum" :default "NewEnumerator0") (BaseValue :type "Float (double-precision)"))
  (bind _structout (setmembers `/Game/Dev/Blueprints/Structs/F_BaseStats` :`StructRef` (`BlueprintMapLibrary.Map_Find` (`self.BaseStats`) stat) :`BaseValue` BaseValue))
  (`BlueprintMapLibrary.Map_Add` (`self.BaseStats`) stat _structout))

(fn `SetCurrentStatValue`
  (params (Stat :type "/Game/Dev/Blueprints/Enums/E_Stats Enum" :default "NewEnumerator0") (Value :type "Float (double-precision)"))
  (`BlueprintMapLibrary.Map_Add` (`self.CurrentStats`) Stat Value)
  (`self.OnCurrentStatValueUpdated` Stat Value))

(fn `SetMaxStatValue`
  (params (Stat :type "/Game/Dev/Blueprints/Enums/E_Stats Enum" :default "NewEnumerator0") (MaxValue :type "Float (double-precision)"))
  (bind _structout (setmembers `/Game/Dev/Blueprints/Structs/F_BaseStats` :`StructRef` (`BlueprintMapLibrary.Map_Find` (`self.BaseStats`) Stat) :`MaxValue` MaxValue))
  (`BlueprintMapLibrary.Map_Add` (`self.BaseStats`) Stat _structout))

(fn `TakeDamage`
  (params (`ınDamage` :type "Float (double-precision)"))
  (locals (`L Damage` :type "Float (double-precision)" :default 0.0))
  (bind _returnvalue (* (`local.L Damage`) -1.0))
  (bind _returnvalue_2 (* (`local.ınDamage`) (/ (`local.ınDamage`) (+ (`local.ınDamage`) (`self.GetCurrentStatValue` "NewEnumerator3")))))
  (set `local.L Damage` (`KismetMathLibrary.FClamp` _returnvalue_2 0.0 _returnvalue_2))
  (`self.ModifyCurrentStatValue` "NewEnumerator1" _returnvalue true)
  (`KismetSystemLibrary.PrintString` (`KismetStringLibrary.Conv_DoubleToString` _returnvalue))
  (if (<= (`self.GetCurrentStatValue` "NewEnumerator1") 0.0)
    (`/Game/Dev/Blueprints/Components/BP_StateComponent.SetState` (`Actor.GetComponentByClass` (`self.GetOwner`) "/Game/Dev/Blueprints/Components/BP_StateComponent.BP_StateComponent_C") (struct :`TagName` "Character.State.Dead"))))